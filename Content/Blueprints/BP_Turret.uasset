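; BP_Turret is a turret that aims and fires BP_Bullet projectiles, though its firing logic is disconnected and Tick is empty.
; The main unused chain traces forward from Body, converts hit distance into gun pitch via the flat-ground ballistic range formula in CalculateAngle, then spawns a bullet with matching launch velocity.
; A second unused chain launches by impulse at zero degrees.
; Both draw predicted projectile paths for debugging.
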(event EventTick
  (params (DeltaSeconds :type Float%20%28single-precision%29)))

(fn ConstructionScript)

(fn CalculateAngle
  (params (DistanceGlobal :type Float%20%28double-precision%29))
  (return (/ (Class|KismetMathLibrary|DegAsin (/ (* DistanceGlobal (LocalVariables|GetGravity)) (* (Variables|Default|GetSpeed) (Variables|Default|GetSpeed)))) 2.0)))