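; Player-controlled gunboat with a mouse-aimed turret and ballistic cannon.
; Mouse input drives a pitch-limited camera, and the turret yaws to match the camera's look direction.
; Left click line-traces along the turret, pitching the barrel using the projectile range formula on hit distance.
; It then spawns a bullet with physics disabled at the arrow and only debug-draws the predicted trajectory, applying no launch velocity.
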(event Collision|EventActorBeginOverlap
  (params (OtherActor :type Actor%20Object%20Reference)))

(event EventBeginPlay
  (bind _returnvalue (Game|GetPlayerCameraManager 0))
  (Variables|/Script/Engine.PlayerCameraManager|SetViewPitchMin _returnvalue -2e+01)
  (Variables|/Script/Engine.PlayerCameraManager|SetViewRollMax _returnvalue 15.0)
  (Variables|/Script/Engine.PlayerCameraManager|SetViewPitchMax _returnvalue 2e+01))

(event Input|MouseEvents|MouseX
  (params (AxisValue :type Float%20%28single-precision%29))
  (Pawn|Input|AddControllerYawInput AxisValue)
  (CallFunction|TurretRotation (Variables|Default|GetTurret)))

(event Input|MouseEvents|MouseY
  (params (AxisValue :type Float%20%28single-precision%29))
  (Pawn|Input|AddControllerPitchInput AxisValue))

(event Input|MouseEvents|LeftMouseButton
  (params (Key :type Key%20Structure :default "None"))
  (bind _turret (Variables|Default|GetTurret))
  (bind _arrow (Variables|Default|GetArrow))
  (bind _returnvalue (Transformation|GetSocketLocation _turret "None"))
  (bind _returnvalue_2 (Transformation|GetSocketLocation _arrow "None"))
  (:Pressed
    (bind (_outhit _returnvalue_3) (Collision|LineTraceByChannel _returnvalue (+ _returnvalue (* (Math|Vector|GetForwardVector _turret) (Variables|Default|GetDistance))) "TraceTypeQuery2" false 0 "Persistent"))
    (if _returnvalue_3
      (bind _angle (CallFunction|CalculateAngle (.Distance (Collision|BreakHitResult _outhit))))
      (Transformation|SetRelativeRotation (Variables|Default|GetBarrel) (Math|Rotator|MakeRotator 0.0 _angle 0.0) false false)
      (bind _returnvalue_4 (Game|SpawnActorfromClass "/Game/Blueprints/BP_Bullet.BP_Bullet_C" (Math|Transform|MakeTransform _returnvalue_2 (Transformation|GetSocketRotation _arrow "None") "1.000000,1.000000,1.000000") "Undefined" "MultiplyWithRoot" 0 0))
      (Physics|SetSimulatePhysics (Variables|/Game/Blueprints/BP_Bullet.BP_Bullet_C|GetSphere _returnvalue_4) false)
      (Class|GameplayStatics|BlueprintPredictProjectilePathAdvanced (Utilities|Struct|MakePredictProjectilePathParams _returnvalue_2 (* (Math|Vector|GetUnitDirection(Vector) (Transformation|GetSocketLocation (Variables|Default|GetTurret) "None") (Transformation|GetWorldLocation (Variables|/Game/Blueprints/BP_Bullet.BP_Bullet_C|GetSphere _returnvalue_4))) (Variables|Default|GetSpeed)) false 0.0 5.0 true "ECC_WorldStatic" "ObjectTypeQuery1" 0 1e+02 0.0 "Persistent" 1.0 false)))))

(fn ConstructionScript)

(fn TurretRotation
  (params (Target :type Scene%20Component%20Object%20Reference))
  (Transformation|SetWorldRotation Target (Math|Rotator|MakeRotator 0.0 0.0 (.yaw (Math|Rotator|FindLookatRotation (Transformation|GetWorldLocation (Variables|Default|GetCamera)) (Transformation|GetWorldLocation Target)))) false false))

(fn CalculateAngle
  (params (Distance :type Float%20%28double-precision%29))
  (return (/ (Class|KismetMathLibrary|DegAsin (/ (* Distance (LocalVariables|GetGravity)) (* (Variables|Default|GetSpeed) (Variables|Default|GetSpeed)))) 2.0)))