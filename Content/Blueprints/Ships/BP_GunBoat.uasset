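; Player-controlled gunboat that drives with physics force and aims a turret-mounted barrel using ballistic math.
; Move input accumulates an acceleration that pushes the hull forward each Tick, while mouse look turns the turret to follow the camera.
; Left click converts the camera trace's hit distance into barrel pitch via the projectile range formula, then draws a predicted trajectory.
; A hidden, non-simulating bullet attached at the muzzle arrow gives the prediction direction; nothing launches it.
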(event Input|EnhancedActionEvents|EnhancedInputActionIA_Move
  (params (ActionValue :type Float%20%28double-precision%29) (ElapsedSeconds :type Float%20%28double-precision%29) (TriggeredSeconds :type Float%20%28double-precision%29) (InputAction :type Input%20Action%20Object%20Reference :default "/Game/IA_Move.IA_Move"))
  (:Triggered
    (Variables|Default|SetAcceleration (+ ActionValue (Variables|Default|GetAcceleration)))))

(event Collision|EventActorBeginOverlap
  (params (OtherActor :type Actor%20Object%20Reference)))

(event EventTick
  (params (DeltaSeconds :type Float%20%28single-precision%29))
  (bind _body (Variables|Default|GetBody))
  (bind _camera (Variables|Default|GetCamera))
  (bind _returnvalue (Transformation|GetWorldLocation _camera))
  (bind _outhit (Collision|LineTraceByChannel _returnvalue (+ _returnvalue (* (Math|Vector|GetForwardVector _camera) (Variables|Default|GetDistance))) "TraceTypeQuery1" false 0 "ForOneFrame"))
  (Variables|Default|SetOut%20Hit _outhit)
  (Class|PrimitiveComponent|AddForceatLocation (Variables|Default|GetBody) (* (Math|Vector|GetForwardVector _body) 1e+03 (Variables|Default|GetAcceleration) (Physics|GetMass _body)) (Transformation|GetWorldLocation (Variables|Default|GetBody)) "None"))

(event EventBeginPlay
  (bind _returnvalue (Game|GetPlayerCameraManager 0))
  (bind _arrow (Variables|Default|GetArrow))
  (Input|AddMappingContext (PlayerController|LocalPlayerSubsystems|GetEnhancedInputLocalPlayerSubsystem (Game|GetPlayerController 0)) "/Game/BP_BoatMappingContext.BP_BoatMappingContext" 0 "(bIgnoreAllPressedKeysUntilRelease=True,bForceImmediately=False,bNotifyUserSettings=False)")
  (Variables|/Script/Engine.PlayerCameraManager|SetViewPitchMin _returnvalue -2e+01)
  (Variables|/Script/Engine.PlayerCameraManager|SetViewRollMax _returnvalue 15.0)
  (Variables|/Script/Engine.PlayerCameraManager|SetViewPitchMax _returnvalue 2e+01)
  (bind _returnvalue_2 (Game|SpawnActorfromClass "/Game/Blueprints/ObjectPool/BP_Bullet.BP_Bullet_C" (Math|Transform|MakeTransform (Transformation|GetSocketLocation _arrow "None") (Transformation|GetSocketRotation _arrow "None") "1.000000,1.000000,1.000000") "Undefined" "MultiplyWithRoot" 0 0))
  (bind _output_get (Variables|Default|SetBullet _returnvalue_2))
  (Transformation|AttachComponentToComponent _output_get (Variables|Default|GetArrow) "None" "KeepWorld" "KeepWorld" "KeepRelative" true)
  (Physics|SetSimulatePhysics (Variables|/Game/Blueprints/ObjectPool/BP_Bullet.BP_Bullet_C|GetSphere _output_get) false)
  (Rendering|SetVisibility (Variables|/Game/Blueprints/ObjectPool/BP_Bullet.BP_Bullet_C|GetSphere _output_get) false false))

(event Input|MouseEvents|MouseX
  (params (AxisValue :type Float%20%28single-precision%29))
  (Pawn|Input|AddControllerYawInput AxisValue)
  (CallFunction|TurretRotation (Variables|Default|GetTurret) (Variables|Default|GetCamera)))

(event Input|MouseEvents|MouseY
  (params (AxisValue :type Float%20%28single-precision%29))
  (Pawn|Input|AddControllerPitchInput AxisValue)
  (Variables|/Script/Engine.SpringArmComponent|SetSocketOffset (Variables|Default|GetSpringArm) (Math|Vector|MakeVector 0.0 0.0 AxisValue)))

(event Input|MouseEvents|LeftMouseButton
  (params (Key :type Key%20Structure :default "None"))
  (:Pressed
    (bind _angle (CallFunction|CalculateAngle (.distance (Variables|Default|GetOut%20Hit))))
    (Transformation|SetRelativeRotation (Variables|Default|GetBarrel) (Math|Rotator|MakeRotator 0.0 _angle 0.0) false false)
    (CallFunction|PredictPath)))

(fn ConstructionScript)

(fn TurretRotation
  (params (Target :type Scene%20Component%20Object%20Reference) (Target1 :type Scene%20Component%20Object%20Reference))
  (Transformation|SetWorldRotation Target (Math|Rotator|MakeRotator 0.0 0.0 (.yaw (Math|Rotator|FindLookatRotation (Transformation|GetWorldLocation Target1) (Transformation|GetWorldLocation Target)))) false false))

(fn CalculateAngle
  (params (Distance :type Float%20%28double-precision%29))
  (return (/ (Class|KismetMathLibrary|DegAsin (/ (* Distance (LocalVariables|GetGravity)) (* (Variables|Default|GetSpeed) (Variables|Default|GetSpeed)))) 2.0)))

(fn PredictPath
  (bind _bullet (Variables|Default|GetBullet))
  (bind _speed (Variables|Default|GetSpeed))
  (bind _turret (Variables|Default|GetTurret))
  (bind _returnvalue (Transformation|GetSocketLocation _turret "None"))
  (bind _sphere (Variables|/Game/Blueprints/ObjectPool/BP_Bullet.BP_Bullet_C|GetSphere _bullet))
  (bind _returnvalue_2 (Transformation|GetWorldLocation _sphere))
  (bind _returnvalue_3 (Math|Vector|GetUnitDirection(Vector) _returnvalue _returnvalue_2))
  (bind _returnvalue_4 (* _returnvalue_3 _speed))
  (Class|GameplayStatics|BlueprintPredictProjectilePathAdvanced (Utilities|Struct|MakePredictProjectilePathParams (Transformation|GetSocketLocation (Variables|Default|GetArrow) "None") _returnvalue_4 false 0.0 5.0 true "ECC_WorldStatic" "ObjectTypeQuery1" 0 1e+02 0.0 "ForDuration" 1.0 false))
  (return _returnvalue_4))