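; Base player boat with a mouse-aimed cannon, driven by physics force and torque on the body from Enhanced Input move and steer actions.
; Each tick, a camera trace's hit distance feeds a ballistic launch-angle formula that eases barrel pitch, while horizontal mouse movement eases turret yaw toward a Scene component.
; Left click launches a physics bullet at BoatStats speed, and right click draws its predicted trajectory as debug.
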(event Input|EnhancedActionEvents|EnhancedInputActionIA_Move
  (params (ActionValue :type Float%20%28double-precision%29) (ElapsedSeconds :type Float%20%28double-precision%29) (TriggeredSeconds :type Float%20%28double-precision%29) (InputAction :type Input%20Action%20Object%20Reference :default "/Game/IA_Move.IA_Move"))
  (Physics|AddForce (Variables|Default|GetBody) (Math|Vector|RotateVector (Math|Vector|MakeVector ActionValue 0.0 0.0) (Transformation|GetSocketRotation (Variables|Default|GetBody) "None")) "None" true))

(event Input|EnhancedActionEvents|EnhancedInputActionIA_Steer
  (params (ActionValue :type Float%20%28double-precision%29) (ElapsedSeconds :type Float%20%28double-precision%29) (TriggeredSeconds :type Float%20%28double-precision%29) (InputAction :type Input%20Action%20Object%20Reference :default "/Game/IA_Steer.IA_Steer"))
  (Class|PrimitiveComponent|AddTorqueinDegrees (Variables|Default|GetBody) (Math|Vector|MakeVector 0.0 0.0 ActionValue) "None" true))

(event EventBeginPlay
  (bind _returnvalue (Game|GetPlayerCameraManager 0))
  (Variables|/Script/Engine.PlayerCameraManager|SetViewPitchMin _returnvalue -2e+01)
  (Variables|/Script/Engine.PlayerCameraManager|SetViewRollMax _returnvalue 15.0)
  (Variables|/Script/Engine.PlayerCameraManager|SetViewPitchMax _returnvalue 2e+01)
  (Input|AddMappingContext (PlayerController|LocalPlayerSubsystems|GetEnhancedInputLocalPlayerSubsystem (Game|GetPlayerController 0)) "/Game/BP_BoatMappingContext.BP_BoatMappingContext" 0 "(bIgnoreAllPressedKeysUntilRelease=True,bForceImmediately=False,bNotifyUserSettings=False)"))

(event Collision|EventActorBeginOverlap
  (params (OtherActor :type Actor%20Object%20Reference)))

(event EventTick
  (params (DeltaSeconds :type Float%20%28single-precision%29))
  (bind _camera (Variables|Default|GetCamera))
  (bind _barrel (Variables|Default|GetBarrel))
  (bind _returnvalue (Transformation|GetWorldLocation _camera))
  (bind _outhit (Collision|LineTraceByChannel _returnvalue (+ _returnvalue (* (Math|Vector|GetForwardVector _camera) (.distance (Variables|Default|GetBoatStats)))) "TraceTypeQuery1" false 0 "ForOneFrame"))
  (bind _angle (CallFunction|CalculateAngle (.distance _outhit) (.bulletspeed (Variables|Default|GetBoatStats))))
  (Transformation|SetRelativeRotation (Variables|Default|GetBarrel) (Math|Rotator|MakeRotator 0.0 (.pitch (Math|Interpolation|RInterpTo (Transformation|GetWorldRotation _barrel) (Math|Rotator|MakeRotator 0.0 _angle (.yaw (Math|Rotator|FindLookatRotation (Transformation|GetWorldLocation _barrel) (Transformation|GetWorldLocation (.hitcomponent _outhit))))) (Utilities|Time|GetWorldDeltaSeconds) 0.5)) 0.0) false false))

(event Input|MouseEvents|MouseX
  (params (AxisValue :type Float%20%28single-precision%29))
  (Pawn|Input|AddControllerYawInput AxisValue)
  (CallFunction|TurretRotation (Variables|Default|GetTurret)))

(event Input|MouseEvents|MouseY
  (params (AxisValue :type Float%20%28single-precision%29))
  (Pawn|Input|AddControllerPitchInput AxisValue))

(event Input|MouseEvents|LeftMouseButton
  (params (Key :type Key%20Structure :default "None"))
  (:Pressed
    (bind _returnvalue (Game|SpawnActorfromClass "/Game/Blueprints/ObjectPool/BP_Bullet.BP_Bullet_C" (Math|Transform|MakeTransform (Transformation|GetWorldLocation (Variables|Default|GetBullet%20REF)) (Transformation|GetSocketRotation (Variables|Default|GetTurret) "None") "1.000000,1.000000,1.000000") "Undefined" "MultiplyWithRoot" 0 0))
    (Physics|SetPhysicsLinearVelocity (Variables|/Game/Blueprints/ObjectPool/BP_Bullet.BP_Bullet_C|GetSphere _returnvalue) (* (Math|Vector|GetUnitDirection(Vector) (Transformation|GetSocketLocation (Variables|Default|GetTurret) "None") (Transformation|GetActorLocation _returnvalue)) (.bulletspeed (Variables|Default|GetBoatStats))) false "None")))

(event Input|MouseEvents|RightMouseButton
  (params (Key :type Key%20Structure :default "None"))
  (bind _bullet_ref (Variables|Default|GetBullet%20REF))
  (bind _returnvalue (Transformation|GetWorldLocation _bullet_ref))
  (:Pressed
    (Class|GameplayStatics|BlueprintPredictProjectilePathAdvanced (Utilities|Struct|MakePredictProjectilePathParams _returnvalue (* (Math|Vector|GetUnitDirection(Vector) (Transformation|GetSocketLocation (Variables|Default|GetTurret) "None") _returnvalue) (.bulletspeed (Variables|Default|GetBoatStats))) false 0.0 3.0 true "ECC_WorldStatic" "ObjectTypeQuery1" 0 1e+02 0.0 "ForDuration" 1.0 false))))

(fn ConstructionScript)

(fn CalculateAngle
  (params (Distance :type Float%20%28double-precision%29) (Bullet%20Speed :type Float%20%28double-precision%29))
  (return (/ (Class|KismetMathLibrary|DegAsin (/ (* Distance (Variables|Default|GetGravity)) (* Bullet%20Speed Bullet%20Speed))) 2.0)))

(fn TurretRotation
  (params (Tuuret :type Static%20Mesh%20Component%20Object%20Reference))
  (Transformation|SetWorldRotation Tuuret (Math|Rotator|MakeRotator 0.0 0.0 (.yaw (Math|Interpolation|RInterpTo (Transformation|GetWorldRotation Tuuret) (Math|Rotator|MakeRotator 0.0 0.0 (.yaw (Math|Rotator|FindLookatRotation (Transformation|GetWorldLocation Tuuret) (Transformation|GetWorldLocation (Variables|Default|GetScene))))) (Utilities|Time|GetWorldDeltaSeconds) 0.5))) false false))