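; BP_BattleShip is a player-controlled battleship whose two turrets turn with the mouse-driven camera.
; On BeginPlay it limits the player camera manager's view pitch and sets a maximum roll.
; Mouse axes feed controller yaw and pitch, and each MouseX event also updates both turrets.
; TurretRotation sets a turret's world yaw along the line from the camera to that turret, zeroing pitch and roll.
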(event EventBeginPlay
  (bind _returnvalue (Game|GetPlayerCameraManager 0))
  (Variables|/Script/Engine.PlayerCameraManager|SetViewPitchMin _returnvalue -2e+01)
  (Variables|/Script/Engine.PlayerCameraManager|SetViewRollMax _returnvalue 15.0)
  (Variables|/Script/Engine.PlayerCameraManager|SetViewPitchMax _returnvalue 2e+01))

(event Collision|EventActorBeginOverlap
  (params (OtherActor :type Actor%20Object%20Reference)))

(event EventTick
  (params (DeltaSeconds :type Float%20%28single-precision%29)))

(event Input|MouseEvents|MouseX
  (params (AxisValue :type Float%20%28single-precision%29))
  (Pawn|Input|AddControllerYawInput AxisValue)
  (CallFunction|TurretRotation (Variables|Default|GetTurret1))
  (CallFunction|TurretRotation (Variables|Default|GetTurret2)))

(event Input|MouseEvents|MouseY
  (params (AxisValue :type Float%20%28single-precision%29))
  (Pawn|Input|AddControllerPitchInput AxisValue))

(fn ConstructionScript)

(fn TurretRotation
  (params (Target :type Scene%20Component%20Object%20Reference))
  (Transformation|SetWorldRotation Target (Math|Rotator|MakeRotator 0.0 0.0 (.yaw (Math|Rotator|FindLookatRotation (Transformation|GetWorldLocation (Variables|Default|GetCamera)) (Transformation|GetWorldLocation Target)))) false false))